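; BP_Claudia is a talkable character Blueprint that shows its Dialog lines on screen, one per Talk event.
; Each Talk increments TalkIndex, then, while the index is no greater than the Dialog length, writes that entry to the widget's TalkText.
; The WBDialogue widget is created lazily for player 0, added to the player screen and reused while valid.
; Nothing here removes the widget or resets the index.
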(event `/Game/BPI_dialogue.Talk`
  (`/Engine/EditorBlueprintResources/StandardMacros.IncrementInt` (`self.talkIndex`)
    (:`  `
      (if (<= (`self.talkIndex`) (`KismetArrayLibrary.Array_Length` (`self.Dialog`)))
        (`self.UI`
          (:`then`
            _)
          (:`else`
            (bind _returnvalue (`|CreateWidget` "/Game/WB+Dialogue.WB+Dialogue_C" (`GameplayStatics.GetPlayerController` 0)))
            (bind _output_get (set `self.UI` _returnvalue))
            (`UserWidget.AddToPlayerScreen` _output_get 0)))
        (`TextBlock.SetText` (`/Game/WB+Dialogue.TalkText` (`self.UI`)) (`KismetTextLibrary.Conv_StringToText` (`|GetArrayItem` (`self.Dialog`) (`self.talkIndex`))))))))

(fn `UserConstructionScript`)