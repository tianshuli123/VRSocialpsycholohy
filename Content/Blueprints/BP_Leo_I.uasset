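; BP_Leo_I is a character actor that shows a name label and dialogue widget when a VR player comes near.
; The construction script writes CharacterName to the TextRender, and BeginPlay caches the widget component's WB_Ignore instance.
; A VRPawn entering the Box reveals the widget and label and calls SetDialogue on that instance.
; Leaving the Box hides both.
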(event `self.ReceiveBeginPlay`
  (bind _aswb_ignore (cast `/Game/UI/WB_Ignore` (`WidgetComponent.GetUserWidgetObject` (`self.Widget`))))
  (set `self.WidgetObject` _aswb_ignore))

(event `self.Box.OnComponentBeginOverlap`
  (params (OverlappedComponent :type "PrimitiveComponent Object Reference") (OtherActor :type "Actor Object Reference") (OtherComp :type "PrimitiveComponent Object Reference") (OtherBodyIndex :type Integer) (bFromSweep :type Boolean) (SweepResult :type "HitResult Structure (by ref)"))
  (cast `/Game/VRTemplate/Blueprints/VRPawn` OtherActor)
  (`SceneComponent.SetVisibility` (`self.Widget`) true false)
  (`SceneComponent.SetVisibility` (`self.TextRender`) true false)
  (`/Game/UI/WB_Ignore.SetDialogue` (`self.WidgetObject`)))

(event `self.Box.OnComponentEndOverlap`
  (params (OverlappedComponent :type "PrimitiveComponent Object Reference") (OtherActor :type "Actor Object Reference") (OtherComp :type "PrimitiveComponent Object Reference") (OtherBodyIndex :type Integer))
  (cast `/Game/VRTemplate/Blueprints/VRPawn` OtherActor)
  (`SceneComponent.SetVisibility` (`self.Widget`) false false)
  (`SceneComponent.SetVisibility` (`self.TextRender`) false false))

(fn `UserConstructionScript`
  (locals (TextRender :type "TextRenderComponent Object Reference") (CharacterName :type Text :default "NSLOCTEXT(\"\", \"947614D74401370C176E0586F3F48F69\", \"Leo\")"))
  (`TextRenderComponent.K2_SetText` (`local.TextRender`) (`local.CharacterName`)))