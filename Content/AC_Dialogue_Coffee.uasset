(fn `Dialogue`
  (`parent.Dialogue`)
  (switch `int` (`self.DialogueTreeIndex`)
    (:`Default`
      (bind (_state _optionindex) (`self.Add Dialogue` "Barista" "Hi, Can What can I get your today?" (`|MakeArray` "Yes" "No" :!type "Text")))
      (switch `/Game/Enum_Dia_state` _state
        (:`NewEnumerator0`
          (switch `int` _optionindex
            (:`0`
              (bind _state_2 (`self.Add Dialogue` "Barista" "Sure!  Here you go!" (`|MakeArray` "Thank you!" :!type "Text")))
              (switch `/Game/Enum_Dia_state` _state_2
                (:`NewEnumerator0`
                  (`self.ClearDialogueProgress`)
                  (`self.CloseConversation`))))
            (:`1`
              (bind _state_3 (`self.Add Dialogue` "Barista" "Thank you for visiting" (`|MakeArray` "Thank you!" :!type "Text")))
              (switch `/Game/Enum_Dia_state` _state_3
                (:`NewEnumerator0`
                  (`self.ClearDialogueProgress`)
                  (`self.CloseConversation`))))))))))