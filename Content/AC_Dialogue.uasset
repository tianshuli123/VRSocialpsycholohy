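; AC_Dialogue is a dialogue component that runs branching conversations through a WB_Dialogue widget and notifies its owner on close.
; Each progression resets the step index and reruns Dialogue, an empty stub for the conversation script.
; AddDialogue replays saved choices from the DialogueProgress map or displays unanswered lines, returning a state and option index.
; Selecting an option records it and triggers another replay, while changing the tree index clears progress.
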(fn `Add Dialogue`
  (params (Speaker :type Text) (Dialogue :type Text) (OptionsText :type "Array of Text"))
  (returns (State :type "/Game/Enum_Dia_state Enum") (OptionIndex :type Integer))
  (bind (_value _returnvalue) (`BlueprintMapLibrary.Map_Find` (`self.DialogueProgress`) (`self.DialogueIndex`)))
  (`/Engine/EditorBlueprintResources/StandardMacros.IncrementInt` (`self.DialogueIndex`)
    (:`  `
      (if _returnvalue
        (return "NewEnumerator0" _value)
        (else
          (`/Game/WB_Dialogue.UpdateDialogueText` (`self.DialogWidget`) 0 (`local.Speaker`) (`local.Dialogue`) (`local.OptionsText`))
          (return "NewEnumerator1" 0))))))

(fn `ClearDialogueProgress`
  (`BlueprintMapLibrary.Map_Clear` (`self.DialogueProgress`)))

(fn `CloseConversation`
  (`Widget.RemoveFromParent` (`self.DialogWidget`))
  (message `/Game/BPI_dialogue.ConversationClosed` (`self.GetOwner`)))

(fn `Dialogue`)

(fn `OpenConversation`
  (bind _returnvalue (`|CreateWidget` "/Game/WB_Dialogue.WB_Dialogue_C" null self))
  (bind _output_get (set `self.DialogWidget` _returnvalue))
  (`UserWidget.AddToViewport` _output_get 0)
  (`self.ProgressDialogue`))

(fn `ProgressDialogue`
  (set `self.DialogueIndex` -1)
  (`self.Dialogue`))

(fn `RemoveDialogueProgress`
  (params (ProgressSteps :type Integer))
  (for _index (range (+ ProgressSteps 1))
    (`BlueprintMapLibrary.Map_Remove` (`self.DialogueProgress`))))

(fn `SetDialogueTreeIndex`
  (params (DialogTreeIndex :type Integer))
  (set `self.DialogueTreeIndex` DialogTreeIndex)
  (`self.ClearDialogueProgress`))

(fn `UpdateSelectedDialogue`
  (params (ProgressIndex :type "Integer (by ref)") (OptionIndex :type "Integer (by ref)"))
  (`BlueprintMapLibrary.Map_Add` (`self.DialogueProgress`) ProgressIndex OptionIndex)
  (`self.ProgressDialogue`))